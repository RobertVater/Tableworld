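; Game instance Blueprint that serves as a lookup point for building definitions stored in the Data_Buildings data table.
; GetBuilding returns the row matching a given ID, handling only the found case.
; GetBuildingsForAgeAndCategory scans every row name and collects the rows whose required age and tile category both match the inputs.
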(fn `getBuilding`
  (params (ID :type "Name (by ref)"))
  (returns (ReturnValue :type "TableBuilding Structure"))
  (bind _returnvalue (`|GetDataTableRow` "/Game/Data/Data_Buildings.Data_Buildings" ID)
    (:`then`
      (return _returnvalue))))

(fn `getBuildingsForAgeAndCategory`
  (params (Age :type "ETableAge Enum" :default "StoneAge") (Category :type "ETableTileCategory Enum" :default "Management"))
  (returns (ReturnValue :type "Array of TableBuilding Structure"))
  (locals (Buildings :type "Array of TableBuilding Structure"))
  (bind _outrownames (`DataTableFunctionLibrary.GetDataTableRowNames` "/Game/Data/Data_Buildings.Data_Buildings"))
  (for _array_element _outrownames
    (bind _returnvalue (`|GetDataTableRow` "/Game/Data/Data_Buildings.Data_Buildings" _array_element)
      (:`then`
        (bind (_icon _name _tooltip _tileclass _requiredage _tilecategory) (break `TableBuilding` _returnvalue))
        (if (and (`|EnumEquality` Age _requiredage) (`|EnumEquality` Category _tilecategory))
          (`KismetArrayLibrary.Array_Add` (`local.Buildings`) _returnvalue)))))
  (return (`local.Buildings`)))